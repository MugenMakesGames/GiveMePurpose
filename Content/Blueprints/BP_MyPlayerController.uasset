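; Player controller that creates the main screen widget, drives NPC spawning and toggles an info screen.
; On BeginPlay it sets game-only input and caches the level's BP_NPCSpawningManager.
; C asks the manager to spawn and move an NPC, printing a debug message if the first value in its message map is false.
; G flip-flops WBP_InfoScreen, restoring game-only input on close; GetCurrentNPC is an empty stub.
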(event `self.ReceiveBeginPlay`
  (`|ExecutionSequence`
    (:`then_0`
      (bind _returnvalue (`|CreateWidget` "/Game/Blueprints/Widgets/WBP_MainScreen.WBP_MainScreen_C"))
      (`UserWidget.AddToViewport` _returnvalue 0)
      (`WidgetBlueprintLibrary.SetInputMode_GameOnly` self))
    (:`then_1`
      (bind _returnvalue_2 (`GameplayStatics.GetActorOfClass` "/Game/Blueprints/NPC/BP_NPCSpawningManager.BP_NPCSpawningManager_C"))
      (set `self.NPCSpawningManagerClass` _returnvalue_2))))

(event `Key|C`
  (params (Key :type "Key Structure"))
  ;[0.1413 0.15 0.04143 0.5] Spawning the NPC's
  ;;[0.09087 0.15 0.06683 0.5] Spawning in the NPC if the last one has passed the cam waypoint
  (:`Pressed`
    (`/Game/Blueprints/NPC/BP_NPCSpawningManager.SpawnNPCAndMoveToWaypoint` (`self.NPCSpawningManagerClass`))
    (bind _hascurrentnpcpassedcam_ (message `/Game/Blueprints/Interfaces/BPI_MainInterface.GetCurrentNPC` (`self.NPCSpawningManagerClass`)))
    (if (not (`.Value` (`BlueprintMapLibrary.Map_GetKeyValueByIndex` _hascurrentnpcpassedcam_)))
      (`KismetSystemLibrary.PrintString` "HAS NOT GOT PURPOSE YET"))))

(event `Key|G`
  (params (Key :type "Key Structure"))
  ;[0.1413 0.15 0.04143 0.5] Spawning the NPC's
  ;;[0.02647 0.1008 0.15 0.5] Displaying the info screen and removing it on G press
  (:`Pressed`
    (`/Engine/EditorBlueprintResources/StandardMacros.FlipFlop`
      (:`A`
        (bind _returnvalue (`|CreateWidget` "/Game/Blueprints/Widgets/WBP_InfoScreen.WBP_InfoScreen_C"))
        (`UserWidget.AddToViewport` _returnvalue 0))
      (:`B`
        (`WidgetBlueprintLibrary.SetInputMode_GameOnly` self)
        (set `self.bShowMouseCursor` false)
        (`Widget.RemoveFromParent` _returnvalue)))))

(fn `GetCurrentNPC`
  (returns (`HasCurrentNPCPassedCam?` :type "Map of /Game/Blueprints/NPC/BP_NPC Object Reference to Boolean"))
  (return))

(fn `UserConstructionScript`)